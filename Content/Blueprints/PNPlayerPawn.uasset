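; Player character Blueprint with camera-relative movement, sprinting, a coin count and a scroll goal.
; A half-second looping timer drops a coin while horizontal speed is at sprint level, spawning it at a mesh socket with a randomly rotated impulse.
; Any damage triggers one-time death with ragdoll and drops all coins.
; Obtaining the scroll stops movement and prints a goal message after a delay; the C key adds a coin.
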(event `self.ReceiveBeginPlay`
  (set `CharacterMovementComponent.MaxWalkSpeed` (`self.GroundWalkSpeed`) (`self.CharacterMovement`))
  (`KismetSystemLibrary.K2_SetTimer` null "CheckSprintRisk" 0.5 true))

(event `self.ReceiveActorBeginOverlap`
  (params (OtherActor :type "Actor Object Reference")))

(event `self.ReceiveTick`
  (params (DeltaSeconds :type "Float (single-precision)")))

(event `InputAxis|MoveForward`
  (params (AxisValue :type "Float (single-precision)"))
  ;[1 1 1] キャラ操作処理
  (`self.AddMovementInput` (`/Game/Blueprints/PNFuncLibrary.FlattenDirection` (`SceneComponent.GetForwardVector` (`self.Camera`))) AxisValue))

(event `InputAxis|MoveRight`
  (params (AxisValue :type "Float (single-precision)"))
  ;[1 1 1] キャラ操作処理
  (`self.AddMovementInput` (`SceneComponent.GetRightVector` (`self.Camera`)) AxisValue))

(event `InputAction|Sprint`
  (bind _charactermovement (`self.CharacterMovement`))
  ;[1 1 1] キャラ操作処理
  (:`Pressed`
    (set `CharacterMovementComponent.MaxWalkSpeed` (`self.GroundSprintSpeed`) _charactermovement))
  (:`Released`
    (set `CharacterMovementComponent.MaxWalkSpeed` (`self.GroundWalkSpeed`) _charactermovement)))

(event `InputAxis|LookUp`
  (params (AxisValue :type "Float (single-precision)"))
  ;[1 1 1] キャラ操作処理
  (`self.AddControllerPitchInput` AxisValue))

(event `InputAxis|LookRight`
  (params (AxisValue :type "Float (single-precision)"))
  ;[1 1 1] キャラ操作処理
  (`self.AddControllerYawInput` AxisValue))

(event `self.ReceiveAnyDamage`
  (params (Damage :type "Float (single-precision)") (DamageType :type "DamageType Object Reference") (InstigatedBy :type "Controller Object Reference") (DamageCauser :type "Actor Object Reference"))
  (`/Engine/EditorBlueprintResources/StandardMacros.DoOnce` false
    (:`Completed`
      (`|ExecutionSequence`
        (:`then_0`
          (`KismetSystemLibrary.PrintString` "Death")
          (`CharacterMovementComponent.DisableMovement` (`self.CharacterMovement`))
          (`self.SetLifeSpan` 5.0)
          (`PrimitiveComponent.SetSimulatePhysics` (`self.Mesh`) true))
        (:`then_1`
          (`self.DropAllCoin`))))))

(event `Key|C`
  (:`Pressed`
    (`self.AddCoin` 1)))

(event `ObtainScroll`
  (`CharacterMovementComponent.DisableMovement` (`self.CharacterMovement`))
  (set `self.HasScroll` true)
  (`KismetSystemLibrary.Delay` 5.0)
  (`KismetSystemLibrary.PrintString` "Goal!!"))

(event `DropAllCoin`
  (while (> (`self.NumOfCoins`) 0)
    (`self.DropCoin`)))

(fn `AddCoin`
  (params (Num :type Integer :default 0))
  (set `self.NumOfCoins` (+ (`self.NumOfCoins`) Num)))

(fn `CheckSprintRisk`
  (if (>= (`/Game/Blueprints/PNActorMacroLibrary.GetFlatSpeed`) (`self.GroundSprintSpeed`))
    (`self.DropCoin`)))

(fn `DropCoin`
  (if (>= (`self.NumOfCoins`) 1)
    (set `self.NumOfCoins` (- (`self.NumOfCoins`) 1))
    (bind _returnvalue (`|SpawnActorFromClass` "/Game/Blueprints/BPCoin.BPCoin_C" (`SceneComponent.GetSocketTransform` (`self.Mesh`) "CoinSpawnPoint" "RTS_World")))
    (`PrimitiveComponent.SetSimulatePhysics` _returnvalue true)
    (`PrimitiveComponent.AddImpulse` _returnvalue (`KismetMathLibrary.RotateAngleAxis` (`KismetMathLibrary.MakeVector` 200.0 0.0 200.0) (`KismetMathLibrary.RandomFloatInRange` 0.0 360.0) (0.0 0.0 1.0)) "None" true)))

(fn `GetCoinNum`
  (returns (`return value` :type Integer))
  (return (`self.NumOfCoins`)))

(fn `UserConstructionScript`)